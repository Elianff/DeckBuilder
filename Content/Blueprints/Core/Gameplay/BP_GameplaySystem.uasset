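; Gameplay system actor that manages which sprites occupy the tiles of a grid.
; Add and remove functions maintain the SpritesOnGrid collection, with optional destruction on removal, and both route through SetSpriteIndexOnGrid.
; That function clears the old tile's occupant, writes the sprite into the new tile's data and moves it above that tile.
; A sentinel index marks off-grid sprites, and indices without a tile send sprites far out of view.
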(event EventBeginPlay)

(event Collision|EventActorBeginOverlap
  (params (OtherActor :type Actor%20Object%20Reference)))

(event EventTick
  (params (DeltaSeconds :type Float%20%28single-precision%29)))

(fn ConstructionScript)

(fn AddSpriteonGrid
  (params (Sprite :type BP%20Sprite%20Object%20Reference) (Index :type Int%20Point%20Structure))
  (Utilities|Array|Add (Variables|Default|GetSpritesOnGrid) Sprite)
  (CallFunction|SetSpriteIndexonGrid Sprite Index))

(fn RemoveSpritefromGrid
  (params (Sprite :type BP%20Sprite%20Object%20Reference) (DestroySprite :type Boolean))
  (Utilities|Array|RemoveItem (Variables|Default|GetSpritesOnGrid) Sprite)
  (CallFunction|SetSpriteIndexonGrid Sprite (Utilities|Struct|MakeIntPoint -999 -999))
  (if DestroySprite
    (Actor|DestroyActor Sprite)))

(fn SetSpriteIndexonGrid
  (params (Sprite :type BP%20Sprite%20Object%20Reference) (Index :type Int%20Point%20Structure))
  (Utilities|FlowControl|Sequence
    (:then_0
      (if (!= (Variables|/Game/Blueprints/Core/Sprites/BP_Sprite.BP_Sprite_C|GetIndex Sprite) Index)
        (Utilities|FlowControl|Sequence
          (:then_0
            (bind _output_get (LocalVariables|SetPreviousTile (.Value (Utilities|Map|Find (Variables|/Game/Blueprints/Core/Grid/BP_Grid.BP_Grid_C|GetGridTiles (Variables|Default|GetGrid)) (Variables|/Game/Blueprints/Core/Sprites/BP_Sprite.BP_Sprite_C|GetIndex Sprite)))))
            (if (== (Utilities|Struct|BreakS_TileData _output_get) Sprite)
              (bind _structout (Utilities|Struct|SetmembersinS_TileData (LocalVariables|GetPreviousTile)))
              (Utilities|Map|Add (Variables|/Game/Blueprints/Core/Grid/BP_Grid.BP_Grid_C|GetGridTiles (Variables|Default|GetGrid)) (Utilities|Struct|BreakS_TileData _structout) _structout)))
          (:then_1
            (Variables|/Game/Blueprints/Core/Sprites/BP_Sprite.BP_Sprite_C|SetIndex Sprite Index)
            (if (!= Index (Utilities|Struct|MakeIntPoint -999 -999))
              (bind _structout_2 (Utilities|Struct|SetmembersinS_TileData (.Value (Utilities|Map|Find (Variables|/Game/Blueprints/Core/Grid/BP_Grid.BP_Grid_C|GetGridTiles (Variables|Default|GetGrid)) Index)) Sprite))
              (Utilities|Map|Add (Variables|/Game/Blueprints/Core/Grid/BP_Grid.BP_Grid_C|GetGridTiles (Variables|Default|GetGrid)) (Utilities|Struct|BreakS_TileData _structout_2) _structout_2))))))
    (:then_1
      (Transformation|SetActorLocation Sprite (+ (select (.ReturnValue (Utilities|Map|Find (Variables|/Game/Blueprints/Core/Grid/BP_Grid.BP_Grid_C|GetGridTiles (Variables|Default|GetGrid)) Index)) (.location (Utilities|Struct|BreakS_TileData (.Value (Utilities|Map|Find (Variables|/Game/Blueprints/Core/Grid/BP_Grid.BP_Grid_C|GetGridTiles (Variables|Default|GetGrid)) Index)))) "-99999.000000,-99999.000000,-99999.000000") "0.000000,0.000000,170.000000") false false))))