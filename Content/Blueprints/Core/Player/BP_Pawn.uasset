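; BP_Pawn is a player-controlled camera pawn that pans and zooms on a spring arm.
; On BeginPlay it seeds its target location and zoom and registers the default Enhanced Input mapping context.
; Move input shifts the target along the actor's forward and right vectors, while zoom input adjusts a clamped target arm length.
; Tick smoothly interpolates the actor location and arm length toward those targets.
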(event Input|EnhancedActionEvents|EnhancedInputActionIA_Camera_Zoom
  (params (ActionValue :type Float%20%28double-precision%29) (ElapsedSeconds :type Float%20%28double-precision%29) (TriggeredSeconds :type Float%20%28double-precision%29) (InputAction :type Input%20Action%20Object%20Reference :default "/Game/Blueprints/Core/Player/Inputs/IA_Camera_Zoom.IA_Camera_Zoom"))
  (Variables|Default|SetDesiredZoom (Math|Float|Clamp(Float) (+ (* ActionValue 4e+01) (Variables|Default|GetDesiredZoom)) 1e+02 1.6e+03)))

(event Input|EnhancedActionEvents|EnhancedInputActionIA_Camera_Move
  (params (ActionValue :type Vector%202D%20Structure) (ElapsedSeconds :type Float%20%28double-precision%29) (TriggeredSeconds :type Float%20%28double-precision%29) (InputAction :type Input%20Action%20Object%20Reference :default "/Game/Blueprints/Core/Player/Inputs/IA_Camera_Move.IA_Camera_Move"))
  (bind _returnvalue (Math|Vector2D|Normalize2D ActionValue))
  (Variables|Default|SetDesiredLocation (+ (Variables|Default|GetDesiredLocation) (* (Transformation|GetActorForwardVector) (* (.x _returnvalue) 2e+01)) (* (Transformation|GetActorRightVector) (* (.y _returnvalue) 2e+01)))))

(event EventBeginPlay
  (bind _returnvalue (Components|GetOwner))
  (bind _asplayer_controller (Utilities|Casting|CastToPlayerController _returnvalue))
  (bind _returnvalue_2 (PlayerController|LocalPlayerSubsystems|GetEnhancedInputLocalPlayerSubsystem _asplayer_controller))
  (Variables|Default|SetDesiredLocation (Transformation|GetActorLocation))
  (Variables|Default|SetDesiredZoom (Variables|/Script/Engine.SpringArmComponent|GetTargetArmLength (Variables|Default|GetSpringArm)))
  (Utilities|IsValid _returnvalue_2
    (:Is%20Valid
      (Input|AddMappingContext _returnvalue_2 "/Game/Blueprints/Core/Player/Inputs/IMC_Default.IMC_Default" 0 "(bIgnoreAllPressedKeysUntilRelease=True,bForceImmediately=False,bNotifyUserSettings=False)"))))

(event Collision|EventActorBeginOverlap
  (params (OtherActor :type Actor%20Object%20Reference)))

(event EventTick
  (params (DeltaSeconds :type Float%20%28single-precision%29))
  (bind _springarm (Variables|Default|GetSpringArm))
  (Variables|/Script/Engine.SpringArmComponent|SetTargetArmLength _springarm (Math|Interpolation|FInterpTo (Variables|/Script/Engine.SpringArmComponent|GetTargetArmLength _springarm) (Variables|Default|GetDesiredZoom) (Utilities|Time|GetWorldDeltaSeconds) 2.0))
  (Transformation|SetActorLocation (Math|Interpolation|VInterpTo (Transformation|GetActorLocation) (Variables|Default|GetDesiredLocation) (Utilities|Time|GetWorldDeltaSeconds) 5.0) false false))

(fn ConstructionScript)