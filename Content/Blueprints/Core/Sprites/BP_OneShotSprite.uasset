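; BP_OneShotSprite is an actor that plays a flipbook animation once and then removes itself, suited to short-lived sprite effects.
; The construction script and BeginPlay both apply the Flipbook variable to the Sprite component and turn looping off.
; BeginPlay also binds the component's finished-playing event, which destroys the actor when the animation ends.
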(event Custom|OnFinishedPlaying_Event
  (Actor|DestroyActor))

(event EventBeginPlay
  (bind _sprite (Variables|Default|GetSprite))
  (Sprite|SetFlipbook _sprite (Variables|Default|GetFlipbook))
  (Components|Timeline|SetLooping _sprite false)
  (EventDispatchers|AssignOnFinishedPlaying _sprite (delegate Custom|OnFinishedPlaying_Event)))

(event Collision|EventActorBeginOverlap
  (params (OtherActor :type Actor%20Object%20Reference)))

(event EventTick
  (params (DeltaSeconds :type Float%20%28single-precision%29)))

(fn ConstructionScript
  (bind _sprite (Variables|Default|GetSprite))
  (Sprite|SetFlipbook _sprite (Variables|Default|GetFlipbook))
  (Components|Timeline|SetLooping _sprite false))