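; BP_actions resolves card actions on the tile grid and adds each action's point value to the controller's EarthHealth.
; RunAction dispatches on action type to add cards, remove, replace or spawn sprites, change terrain, enlarge the hand, skip timers or water trees into their next growth stage.
; Spreading actions instead scan neighbouring tiles within AdjacentRange, rolling a percent chance for fire removal or bonus cards.
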(fn RunAction
  (params (typeOfAction :type e_TypeOfAction%20Enum :default "NewEnumerator0") (actions :type S%20Actions%20Structure) (GameplaySystem :type BP%20Gameplay%20System%20Object%20Reference) (Player%20Actions :type BP%20Player%20Actions%20Object%20Reference) (Sprite :type BP%20Sprite%20Object%20Reference) (Index :type Int%20Point%20Structure) (cardInfo :type S%20Card%20Info%20Structure))
  (bind (_cardtype _cardtypeofinteractablegrid _frequency _xhowmanyturns_ _untilwhichround _typeofaction_ _whatcard_ _addallcards_ _whatterraintochangeto _howmanycardsaffectedbyaction_ _whatisbeingspread _spreadpercent _doesgrowthphasematter_ _requiredgrowthphase _pointvalue) (Utilities|Struct|Breaks_actions actions))
  (bind _returnvalue (Utilities|Enum|ByteToEnume_TypeOfAction typeOfAction))
  (bind _grid (Variables|/Game/Blueprints/Core/Gameplay/BP_GameplaySystem.BP_GameplaySystem_C|GetGrid GameplaySystem))
  (bind _spriteontile (CallFunction|GetSpriteonTile _grid Index))
  (if (Utilities|Enum|NotEqual(Enum) _whatisbeingspread "NewEnumerator3")
    (CallFunction|CheckAdjacentIndices Index Player%20Actions GameplaySystem Sprite actions cardInfo)
    (if true :!label _label
      (bind _asbp_card_controller (Utilities|Casting|CastToBP_CardController (Game|GetPlayerController 0)))
      (Development|PrintString 0 (Utilities|String|ToString(Float) _pointvalue))
      (Variables|/Game/CardUI/BP_CardController.BP_CardController_C|SetearthHealth _asbp_card_controller (+ (Variables|/Game/CardUI/BP_CardController.BP_CardController_C|GetearthHealth _asbp_card_controller) _pointvalue)))
    (else
      (bind _asbp_card_controller_2 (Utilities|Casting|CastToBP_CardController (Game|GetPlayerController 0)))
      (if (Utilities|Enum|Equal(Enum) _returnvalue "NewEnumerator0")
        (CallFunction|AddCardAction _whatcard_ (Variables|/Game/CardUI/BP_CardController.BP_CardController_C|GetcardHand _asbp_card_controller_2) _addallcards_ _howmanycardsaffectedbyaction_)
        (goto _label)
        (elif (Utilities|Enum|Equal(Enum) _returnvalue "NewEnumerator1")
          (CallFunction|RemoveItemonGrid GameplaySystem Sprite)
          (goto _label)
          (elif (not (Utilities|Enum|Equal(Enum) _returnvalue "NewEnumerator2"))
            (if (Utilities|Enum|Equal(Enum) _returnvalue "NewEnumerator3")
              (CallFunction|ReplaceItemonGrid GameplaySystem actions Player%20Actions Sprite _whatterraintochangeto Index)
              (goto _label)
              (elif (Utilities|Enum|Equal(Enum) _returnvalue "NewEnumerator8")
                (CallFunction|Spawn Player%20Actions Index cardInfo _whatterraintochangeto)
                (goto _label)
                (elif (Utilities|Enum|Equal(Enum) _returnvalue "NewEnumerator9")
                  (CallFunction|AddCardSize)
                  (goto _label)
                  (elif (Utilities|Enum|Equal(Enum) _returnvalue "NewEnumerator5")
                    (CallFunction|SkipTimer Index)
                    (goto _label)
                    (elif (Utilities|Enum|Equal(Enum) _returnvalue "NewEnumerator10")
                      (CallFunction|TerrainChanger :Gameplay%20System GameplaySystem :Index Index)
                      (goto _label)
                      (elif (Utilities|Enum|Equal(Enum) _returnvalue "NewEnumerator7")
                        (Utilities|IsValid _spriteontile
                          (:Is%20Valid
                            (CallFunction|WaterCardAction _spriteontile cardInfo Player%20Actions)
                            (goto _label)))))))))))))))

(fn AddCardAction
  (params (Cards%20to%20Add :type Array%20of%20E_CardType%20Enums :default "NewEnumerator1") (Card%20Hand :type Widget%20Card%20Hand%20Object%20Reference) (AddAllCards :type Boolean) (HowManyCardsToAdd :type Integer))
  (bind (_howmanycardstoadd _allofthemfit) (CallFunction|HowManyCardstoAdd (Utilities|Array|Length Cards%20to%20Add)))
  (if AddAllCards
    (if _allofthemfit
      (CallFunction|AddingCardsThatFit Cards%20to%20Add Card%20Hand)
      (else
        (CallFunction|AddingAllCardsThatDontAllFit Cards%20to%20Add _howmanycardstoadd Card%20Hand)))
    (else
      (CallFunction|AddRandomCard Cards%20to%20Add HowManyCardsToAdd Card%20Hand))))

(fn HowManyCardstoAdd
  (params (length :type Integer))
  (bind _asbp_card_controller (Utilities|Casting|CastToBP_CardController (Game|GetPlayerController 0)))
  (if (<= length (- (Variables|/Game/CardUI/BP_CardController.BP_CardController_C|GetmaxHandSize _asbp_card_controller) (Variables|/Game/CardUI/BP_CardController.BP_CardController_C|GetAmtOfCards _asbp_card_controller)))
    (return length true)
    (else
      (return (- length (- (Variables|/Game/CardUI/BP_CardController.BP_CardController_C|GetmaxHandSize _asbp_card_controller) (Variables|/Game/CardUI/BP_CardController.BP_CardController_C|GetAmtOfCards _asbp_card_controller))) false))))

(fn AddingCardsThatFit
  (params (CardsToAdd :type Array%20of%20E_CardType%20Enums :default "NewEnumerator1") (CardHand :type Widget%20Card%20Hand%20Object%20Reference))
  (for _array_element CardsToAdd
    (bind _cardinfo (CallFunction|GetDefaultCardInfofromCardType _array_element))
    (Default|AddCard CardHand _cardinfo)))

(fn AddingAllCardsThatDontAllFit
  (params (CardsToAdd :type Array%20of%20E_CardType%20Enums :default "NewEnumerator1") (HowManyCardsToAdd :type Integer) (CardHand :type Widget%20Card%20Hand%20Object%20Reference))
  (bind (_array_element _array_index) (Utilities|Array|ForEachLoopwithBreak CardsToAdd :!label _label)
    (:LoopBody
      (if (== _array_index HowManyCardsToAdd)
        (goto _label Break)
        (else
          (bind _cardinfo (CallFunction|GetDefaultCardInfofromCardType _array_element))
          (Default|AddCard CardHand _cardinfo))))))

(fn AddRandomCard
  (params (CardsToAdd :type Array%20of%20E_CardType%20Enums :default "NewEnumerator1") (HowManyCardsToAdd :type Integer) (CardHand :type Widget%20Card%20Hand%20Object%20Reference))
  (for _index (range 0 (- HowManyCardsToAdd 1))
    (bind _cardinfo (CallFunction|GetDefaultCardInfofromCardType (.OutItem (Utilities|Array|Random CardsToAdd))))
    (Default|AddCard CardHand _cardinfo)))

(fn ReplaceItemonGrid
  (params (GameplaySystem :type BP%20Gameplay%20System%20Object%20Reference) (Actions :type S%20Actions%20Structure) (PlayerActions :type BP%20Player%20Actions%20Object%20Reference) (Sprite :type BP%20Sprite%20Object%20Reference) (TerrainToSetTo :type S%20Terrain%20Type%20Structure) (Index :type Int%20Point%20Structure))
  (Default|GetTileIndexUnderCursor (Variables|/Game/Blueprints/Core/Player/BP_PlayerActions.BP_PlayerActions_C|GetGrid PlayerActions))
  (Default|RemoveSpritefromGrid GameplaySystem Sprite true)
  (bind _cardinfo (CallFunction|GetDefaultCardInfofromCardType (.OutItem (Utilities|Array|Random (.WhatCard? (Utilities|Struct|Breaks_actions Actions))))))
  (CallFunction|Spawn PlayerActions Index _cardinfo TerrainToSetTo))

(fn RemoveItemonGrid
  (params (Gameplay%20System :type BP%20Gameplay%20System%20Object%20Reference) (Sprite :type BP%20Sprite%20Object%20Reference))
  (Default|RemoveSpritefromGrid Gameplay%20System Sprite true))

(fn CheckAdjacentIndices
  (params (Index :type Int%20Point%20Structure) (Player%20Actions :type BP%20Player%20Actions%20Object%20Reference) (Gameplay%20System :type BP%20Gameplay%20System%20Object%20Reference) (Sprite :type BP%20Sprite%20Object%20Reference) (Actions :type S%20Actions%20Structure) (Card%20Info :type S%20Card%20Info%20Structure))
  (bind (_x _y) (Utilities|Struct|BreakIntPoint Index))
  (bind (_cardtype _cardtypeofinteractablegrid _frequency _xhowmanyturns_ _untilwhichround _typeofaction_ _whatcard_ _addallcards_ _whatterraintochangeto _howmanycardsaffectedbyaction_ _whatisbeingspread _spreadpercent) (Utilities|Struct|Breaks_actions Actions))
  (LocalVariables|SetlowerX (- _x (LocalVariables|GetAdjacentRange)))
  (LocalVariables|SetUpperX (+ _x (LocalVariables|GetAdjacentRange)))
  (LocalVariables|SetlowerY (- _y (LocalVariables|GetAdjacentRange)))
  (LocalVariables|SetUpperY (+ _y (LocalVariables|GetAdjacentRange)))
  (for _index (range (LocalVariables|GetlowerX) (LocalVariables|GetUpperX))
    (for _index_2 (range (LocalVariables|GetlowerY) (LocalVariables|GetUpperY))
      (if (Default|IsIndexValid (Variables|/Game/Blueprints/Core/Gameplay/BP_GameplaySystem.BP_GameplaySystem_C|GetGrid Gameplay%20System) (Utilities|Struct|MakeIntPoint _index _index_2))
        (CallFunction|AdjacentAction _whatisbeingspread _spreadpercent (.CardCategory (Utilities|Struct|BreakS_CardInfo Card%20Info)) (Utilities|Struct|MakeIntPoint _index _index_2) Card%20Info Player%20Actions Sprite Gameplay%20System)))))

(fn AdjacentAction
  (params (what%20is%20being%20spread :type e_adjacent%20Enum :default "NewEnumerator3") (spread%20percent :type Float%20%28double-precision%29) (Card%20Category :type e_typeCategory%20Enum :default "NewEnumerator0") (Index :type Int%20Point%20Structure) (Card%20Info :type S%20Card%20Info%20Structure) (Player%20Actions :type BP%20Player%20Actions%20Object%20Reference) (Sprite :type BP%20Sprite%20Object%20Reference) (Gameplay%20System :type BP%20Gameplay%20System%20Object%20Reference))
  (if (Utilities|Enum|Equal(Enum) what%20is%20being%20spread "NewEnumerator0")
    (CallFunction|SpreadingFire spread%20percent Index Gameplay%20System Sprite)
    (elif (Utilities|Enum|Equal(Enum) what%20is%20being%20spread "NewEnumerator5")
      (bind _effect_can_trigger (CallFunction|RandomPercent spread%20percent))
      (if _effect_can_trigger
        (bind _asbp_card_controller (Utilities|Casting|CastToBP_CardController (Game|GetPlayerController 0)))
        (CallFunction|AddCardAction (Utilities|Array|MakeArray "NewEnumerator10") (Variables|/Game/CardUI/BP_CardController.BP_CardController_C|GetcardHand _asbp_card_controller) true)))))

(fn SpreadingFire
  (params (Spread%20Percent :type Float%20%28double-precision%29) (Index :type Int%20Point%20Structure) (Gameplay%20System :type BP%20Gameplay%20System%20Object%20Reference) (Sprite :type BP%20Sprite%20Object%20Reference))
  (bind _terrain (CallFunction|CheckGrid'sTerrain Index))
  (bind _effect_can_trigger (CallFunction|RandomPercent Spread%20Percent))
  (if (and _effect_can_trigger (Utilities|Enum|Equal(Enum) (.Category (Utilities|Struct|Breaks_TerrainType _terrain)) "NewEnumerator0"))
    (CallFunction|RemoveItemonGrid Gameplay%20System Sprite)))

(fn RandomPercent
  (params (Percent :type Float%20%28double-precision%29))
  (bind _output_get (LocalVariables|SetrandomFloat (Math|Random|RandomFloatinRange 1.0 1e+02)))
  (if (>= Percent _output_get)
    (return true)
    (else
      (return false))))

(fn AddCardSize
  (bind _asbp_card_controller (Utilities|Casting|CastToBP_CardController (Game|GetPlayerController 0)))
  (Variables|/Game/CardUI/BP_CardController.BP_CardController_C|SetmaxHandSize _asbp_card_controller (+ (Variables|/Game/CardUI/BP_CardController.BP_CardController_C|GetmaxHandSize _asbp_card_controller) 1)))

(fn SkipTimer
  (params (Index :type Int%20Point%20Structure))
  (bind _asbp_card_controller (Utilities|Casting|CastToBP_CardController (Game|GetPlayerController 0)))
  (Utilities|Map|Add (Utilities|Struct|Breaks_frequencyMap (Variables|/Game/CardUI/BP_CardController.BP_CardController_C|GetfreqMap _asbp_card_controller)) Index (Utilities|Struct|Makes_FreqAndXContainer (.Frequency (Utilities|Struct|Breaks_FreqAndXContainer (.Value (Utilities|Map|Find (Utilities|Struct|Breaks_frequencyMap (Variables|/Game/CardUI/BP_CardController.BP_CardController_C|GetfreqMap _asbp_card_controller)) Index)))) (.Action (Utilities|Struct|Breaks_FreqAndXContainer (.Value (Utilities|Map|Find (Utilities|Struct|Breaks_frequencyMap (Variables|/Game/CardUI/BP_CardController.BP_CardController_C|GetfreqMap _asbp_card_controller)) Index)))) (.OriginalX (Utilities|Struct|Breaks_FreqAndXContainer (.Value (Utilities|Map|Find (Utilities|Struct|Breaks_frequencyMap (Variables|/Game/CardUI/BP_CardController.BP_CardController_C|GetfreqMap _asbp_card_controller)) Index)))) (- (.CurrentX (Utilities|Struct|Breaks_FreqAndXContainer (.Value (Utilities|Map|Find (Utilities|Struct|Breaks_frequencyMap (Variables|/Game/CardUI/BP_CardController.BP_CardController_C|GetfreqMap _asbp_card_controller)) Index)))) 1.0) (.UntilWhenWeStop (Utilities|Struct|Breaks_FreqAndXContainer (.Value (Utilities|Map|Find (Utilities|Struct|Breaks_frequencyMap (Variables|/Game/CardUI/BP_CardController.BP_CardController_C|GetfreqMap _asbp_card_controller)) Index)))) (.Actions (Utilities|Struct|Breaks_FreqAndXContainer (.Value (Utilities|Map|Find (Utilities|Struct|Breaks_frequencyMap (Variables|/Game/CardUI/BP_CardController.BP_CardController_C|GetfreqMap _asbp_card_controller)) Index)))) (.GameplaySystem (Utilities|Struct|Breaks_FreqAndXContainer (.Value (Utilities|Map|Find (Utilities|Struct|Breaks_frequencyMap (Variables|/Game/CardUI/BP_CardController.BP_CardController_C|GetfreqMap _asbp_card_controller)) Index)))) (.PlayerActions (Utilities|Struct|Breaks_FreqAndXContainer (.Value (Utilities|Map|Find (Utilities|Struct|Breaks_frequencyMap (Variables|/Game/CardUI/BP_CardController.BP_CardController_C|GetfreqMap _asbp_card_controller)) Index)))) (.Sprite (Utilities|Struct|Breaks_FreqAndXContainer (.Value (Utilities|Map|Find (Utilities|Struct|Breaks_frequencyMap (Variables|/Game/CardUI/BP_CardController.BP_CardController_C|GetfreqMap _asbp_card_controller)) Index)))) (.Index (Utilities|Struct|Breaks_FreqAndXContainer (.Value (Utilities|Map|Find (Utilities|Struct|Breaks_frequencyMap (Variables|/Game/CardUI/BP_CardController.BP_CardController_C|GetfreqMap _asbp_card_controller)) Index)))) (.CardInfo (Utilities|Struct|Breaks_FreqAndXContainer (.Value (Utilities|Map|Find (Utilities|Struct|Breaks_frequencyMap (Variables|/Game/CardUI/BP_CardController.BP_CardController_C|GetfreqMap _asbp_card_controller)) Index)))) (.Grid (Utilities|Struct|Breaks_FreqAndXContainer (.Value (Utilities|Map|Find (Utilities|Struct|Breaks_frequencyMap (Variables|/Game/CardUI/BP_CardController.BP_CardController_C|GetfreqMap _asbp_card_controller)) Index)))))))

(fn RemoveState
  (params (Index :type Int%20Point%20Structure))
  (bind _asbp_card_controller (Utilities|Casting|CastToBP_CardController (Game|GetPlayerController 0)))
  (Utilities|Map|Remove (Utilities|Struct|Breaks_frequencyMap (Variables|/Game/CardUI/BP_CardController.BP_CardController_C|GetfreqMap _asbp_card_controller)) Index)
  (CallFunction|EraseGridStates Index))

(fn InsectAction
  (params (Actions :type S%20Actions%20Structure) (cardHand :type Widget%20Card%20Hand%20Object%20Reference))
  (if (Utilities|Enum|Equal(Enum) (.CardTypeOfInteractableGrid (Utilities|Struct|Breaks_actions Actions)) "NewEnumerator4")
    (bind _effect_can_trigger (CallFunction|RandomPercent 5e+01))
    (if _effect_can_trigger
      (CallFunction|RemoveState)
      (bind _output_get (LocalVariables|SetCardsToAdd (Utilities|Array|MakeArray "NewEnumerator7" "NewEnumerator7")))
      (CallFunction|AddCardAction _output_get cardHand true))))

(fn Spawn
  (params (Player%20Actions :type BP%20Player%20Actions%20Object%20Reference) (Index :type Int%20Point%20Structure) (Card%20Info :type S%20Card%20Info%20Structure) (TerrainToChangeItTo :type S%20Terrain%20Type%20Structure))
  (bind _asbp_card_controller (Utilities|Casting|CastToBP_CardController (Game|GetPlayerController 0)))
  (CallFunction|SetTerrain Index (.Value (Utilities|Map|Find (Variables|/Game/CardUI/BP_CardController.BP_CardController_C|GetGridStatusArray _asbp_card_controller) Index)) TerrainToChangeItTo)
  (Default|OnlySpawnSprite Player%20Actions Index Card%20Info))

(fn WaterCardAction
  (params (Sprite%20On%20Tile :type BP%20Sprite%20Object%20Reference) (Card%20Info :type S%20Card%20Info%20Structure) (Player%20Actions :type BP%20Player%20Actions%20Object%20Reference))
  (bind _sprite (Variables|/Script/Paper2D.PaperCharacter|GetSprite Sprite%20On%20Tile))
  (Utilities|IsValid Sprite%20On%20Tile
    (:Is%20Valid
      (if (Utilities|Enum|Equal(Enum) (.Type (Utilities|Struct|BreakS_CardInfo Card%20Info)) "NewEnumerator0")
        (Default|SpawnOneShotSprite Player%20Actions (Transformation|GetActorLocation Sprite%20On%20Tile) Card%20Info)
        (if (not (Utilities|Enum|Equal(Enum) (Variables|/Game/Blueprints/Core/Sprites/BP_Sprite.BP_Sprite_C|GetGrowthStage Sprite%20On%20Tile) "NewEnumerator2"))
          (Variables|/Game/Blueprints/Core/Sprites/BP_Sprite.BP_Sprite_C|SetGrowthStage Sprite%20On%20Tile (Utilities|Enum|ByteToEnumE_TreeSpriteGrowthStage (Math|Conversions|ToByte(Integer) (+ (Math|Conversions|ToInteger(Byte) (Variables|/Game/Blueprints/Core/Sprites/BP_Sprite.BP_Sprite_C|GetGrowthStage Sprite%20On%20Tile)) 1))))
          (bind _cardinfo (CallFunction|GetDefaultCardInfofromCardType (Variables|/Game/Blueprints/Core/Sprites/BP_Sprite.BP_Sprite_C|GetCardType Sprite%20On%20Tile)))
          (Utilities|IsValid (.Value (Utilities|Map|Find (.TreeGrowthStages (Utilities|Struct|BreakS_CardInfo _cardinfo)) (Variables|/Game/Blueprints/Core/Sprites/BP_Sprite.BP_Sprite_C|GetGrowthStage Sprite%20On%20Tile)))
            (:Is%20Valid
              (Audio|SpawnSound2D 0 "/Game/Sound/SoundEffects/Plants/Grow.Grow" 1.0 1.0 0.0 0)
              (Sprite|SetFlipbook _sprite (.Value (Utilities|Map|Find (.TreeGrowthStages (Utilities|Struct|BreakS_CardInfo _cardinfo)) (Variables|/Game/Blueprints/Core/Sprites/BP_Sprite.BP_Sprite_C|GetGrowthStage Sprite%20On%20Tile))))
              (Components|Timeline|SetLooping _sprite (.IsAnimationLooping (Utilities|Struct|BreakS_CardInfo _cardinfo)))
              (Audio|Components|Audio|Stop _sprite)
              (Components|Timeline|PlayfromStart _sprite))))
        (else
          (Development|PrintString 0 "Not On Seed") ; TODO: replace with sound cue to let player knows there is no seed on tile
        )))))

(fn PlantPhaseChecker
  (params (IsPlantPhaseRequired? :type Boolean) (NeededPhase :type E_TreeSpriteGrowthStage%20Enum :default "NewEnumerator0") (currentPhase :type E_TreeSpriteGrowthStage%20Enum :default "NewEnumerator0"))
  (if IsPlantPhaseRequired?
    (return (Utilities|Enum|Equal(Enum) NeededPhase currentPhase))))