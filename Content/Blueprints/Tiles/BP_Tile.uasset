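; BP_Tile is a single grid tile actor that changes color to show whether it is selected.
; Initialize sets a plane mesh, attaches the tile to its owner and offsets it by Column and Row times the mesh's bounds.
; A dynamic instance of M_Tile, created on BeginPlay and again on mesh setup, drives the Color parameter.
; OnInteract switches between selected and normal colors, returning whether the material was valid.
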(event EventBeginPlay
  (CallFunction|CreateMID))

(event Collision|EventActorBeginOverlap
  (params (OtherActor :type Actor%20Object%20Reference)))

(event EventTick
  (params (DeltaSeconds :type Float%20%28single-precision%29)))

(fn ConstructionScript)

(fn Initialize
  (bind _returnvalue (Components|GetOwner))
  (Utilities|IsValid _returnvalue
    (:Is%20Valid
      (CallFunction|SetMesh)
      (Transformation|AttachActorToActor _returnvalue "None" "SnapToTarget" "SnapToTarget" "KeepRelative" false)
      (bind _returnvalue_2 (CallFunction|CalculateLocation))
      (Transformation|SetActorRelativeLocation _returnvalue_2))))

(fn CalculateLocation
  (bind _tile (Variables|Default|GetTile))
  (bind _boxextent (Collision|GetComponentBounds _tile))
  (bind (_x _y) (Math|Vector|BreakVector _boxextent))
  (return (Math|Vector|MakeVector (* _x (Variables|Default|GetColumn) 2.0) (* _y (Variables|Default|GetRow) 2.0) 0.0)))

(fn CreateMID
  (bind _returnvalue (Rendering|Material|CreateDynamicMaterialInstance (Variables|Default|GetTile) 0 "/Game/Blueprints/Materials/Tiles/M_Tile.M_Tile" "None" :!class /Script/Engine.PrimitiveComponent))
  (bind _output_get (Variables|Material|SetMID _returnvalue))
  (Rendering|Material|SetVectorParameterValue _output_get "Color" (Variables|Color|GetNormalColor) :!class /Script/Engine.MaterialInstanceDynamic))

(fn SetMesh
  (Components|StaticMesh|SetStaticMesh (Variables|Default|GetTile) "/Engine/BasicShapes/Plane.Plane")
  (CallFunction|CreateMID))

(fn OnInteract
  (params (IsSelected :type Boolean))
  (bind _mid (Variables|Material|GetMID)
    (:then
      (Rendering|Material|SetVectorParameterValue _mid "Color" (Math|Color|SelectColor (Variables|Color|GetSelectedColor) (Variables|Color|GetNormalColor) (LocalVariables|GetisSelected)) :!class /Script/Engine.MaterialInstanceDynamic)
      (return true))
    (:else
      (return false))))